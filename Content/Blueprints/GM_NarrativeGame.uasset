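; GM_NarrativeGame is the game mode for a narrative game, relaying game-state and choice events to the HUD.
; Both handlers reach the WBP_HUD widget by casting player controller 0 to PC_NarrativeGame and reading its HUD widget instance.
; A state change switches the HUD view and, for Dialog View, displays a segment.
; A resolved choice passes its success flag to the HUD.
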(event `self.OnGameStateChanged`
  (params (NewState :type "EGameState Enum" :default "EMapView"))
  (bind _aspc_narrative_game (cast `/Game/Blueprints/PC_NarrativeGame` (`GameplayStatics.GetPlayerController` 0)))
  (bind _aswbp_hud (cast `/Game/Blueprints/WBP_HUD` (`NarrativePlayerController.HUDWidgetInstance` _aspc_narrative_game)))
  (`/Game/Blueprints/WBP_HUD.SwitchToView` _aswbp_hud NewState)
  (switch `EGameState` NewState
    (:`EDialogView`
      (`/Game/Blueprints/WBP_HUD.DisplaySegment` _aswbp_hud))))

(event `self.OnChoiceResolved`
  (params (bWasSuccess :type Boolean))
  (bind _aspc_narrative_game (cast `/Game/Blueprints/PC_NarrativeGame` (`GameplayStatics.GetPlayerController` 0)))
  (bind _aswbp_hud (cast `/Game/Blueprints/WBP_HUD` (`NarrativePlayerController.HUDWidgetInstance` _aspc_narrative_game)))
  (`/Game/Blueprints/WBP_HUD.UpdateLastChoiceWasSuccessful` _aswbp_hud bWasSuccess))

(fn `UserConstructionScript`)