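; Player controller for a narrative game that creates and holds the player's main UI widgets.
; On BeginPlay it adds a HUD to the viewport, then creates the map and dialog widgets without displaying them, keeping references to all three.
; It shows the mouse cursor and switches input to UI-only with focus on the HUD, with no Tick logic.
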(event `self.ReceiveBeginPlay`
  (bind _returnvalue (`GameplayStatics.GetPlayerControllerFromID` 0))
  (bind _returnvalue_2 (`|CreateWidget` "/Game/Blueprints/WBP_HUD.WBP_HUD_C" self))
  (`UserWidget.AddToViewport` _returnvalue_2 0)
  (bind _returnvalue_3 (`|CreateWidget` "/Game/Blueprints/WBP_Map.WBP_Map_C" self))
  (set `self.MapWidget` _returnvalue_3)
  (bind _returnvalue_4 (`|CreateWidget` "/Game/Blueprints/WBP_Dialog.WBP_Dialog_C" self))
  (set `self.DialogWidget` _returnvalue_4)
  (set `self.HUDReference` _returnvalue_2)
  (set `PlayerController.bShowMouseCursor` true _returnvalue)
  (`WidgetBlueprintLibrary.SetInputMode_UIOnlyEx` _returnvalue _returnvalue_2))

(fn `UserConstructionScript`)