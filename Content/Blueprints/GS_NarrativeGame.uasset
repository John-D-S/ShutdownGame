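; Narrative game state, by its GS prefix, that starts a new day with a token range matching the chosen difficulty.
; On BeginPlay it casts the game instance to GI_Shutdown and switches on its Difficulty setting.
; Each Easy, Normal or Hard branch passes that level's min and max tokens from the game instance into InitializeNewDay, which is defined outside these graphs.
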(event `self.ReceiveBeginPlay`
  (bind _asgi_shutdown (cast `/Game/Blueprints/GI_Shutdown` (`GameplayStatics.GetGameInstance`)))
  (switch `/Game/Blueprints/Difficulty` (`/Game/Blueprints/GI_Shutdown.Difficulty` _asgi_shutdown)
    (:`NewEnumerator0`
      (`self.InitializeNewDay` (`/Game/Blueprints/GI_Shutdown.EasyMinTokens` _asgi_shutdown) (`/Game/Blueprints/GI_Shutdown.EasyMaxTokens` _asgi_shutdown)))
    (:`NewEnumerator1`
      (`self.InitializeNewDay` (`/Game/Blueprints/GI_Shutdown.NormalMinTokens` _asgi_shutdown) (`/Game/Blueprints/GI_Shutdown.NormalMaxTokens` _asgi_shutdown)))
    (:`NewEnumerator2`
      (`self.InitializeNewDay` (`/Game/Blueprints/GI_Shutdown.HardMinTokens` _asgi_shutdown) (`/Game/Blueprints/GI_Shutdown.HardMaxTokens` _asgi_shutdown)))))

(fn `UserConstructionScript`)